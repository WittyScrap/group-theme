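; Ice projectile actor that freezes what it hits.
; On the first Box hit it sends FreezeObjectMessage to the other actor if that implements BPI_DragonGame, then destroys itself either way.
; On BeginPlay it copies BaseSpeed into the ProjectileMovement initial and max speed, so speed can vary per use, then applies GravityScale after a brief delay.
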(event OnComponentHit(Box)
  (params (HitComponent :type Primitive%20Component%20Object%20Reference) (OtherActor :type Actor%20Object%20Reference) (OtherComp :type Primitive%20Component%20Object%20Reference) (NormalImpulse :type Vector :default "0, 0, 0") (Hit :type Hit%20Result%20Structure%20%28by%20ref%29))
  ;[1 1 1] On hit freeze object
  (Utilities|FlowControl|DoOnce false
    (:Completed
      (Utilities|FlowControl|Sequence
        (:then_0
          (if (Utilities|DoesObjectImplementInterface OtherActor "/Game/Blueprints/Lib/BPI_DragonGame.BPI_DragonGame_C")
            (Class|BPIDragonGame|FreezeObject(Message) OtherActor)))
        (:then_1
          (Actor|DestroyActor))))))

(event EventBeginPlay
  (bind _projectilemovement (Variables|Default|GetProjectileMovement))
  (bind _basespeed (Variables|Default|GetBaseSpeed))
  ;[1 1 1] When spawned allow us to set the projectile speed for different scenarios (ie enemies using fire)
  (Variables|/Script/Engine.ProjectileMovementComponent|SetInitialSpeed _projectilemovement _basespeed)
  (Variables|/Script/Engine.ProjectileMovementComponent|SetMaxSpeed _projectilemovement _basespeed)
  (Utilities|FlowControl|Delay 0.05)
  (Variables|/Script/Engine.ProjectileMovementComponent|SetProjectileGravityScale _projectilemovement (Variables|Default|GetGravityScale)))

(fn ConstructionScript)
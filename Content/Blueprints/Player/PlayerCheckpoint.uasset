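; Checkpoint trigger that saves player progress when its box is overlapped by any actor.
; It saves if no save exists or its GateNum exceeds the saved one, preventing backtracking or repeat triggers from overwriting progress.
; Each save creates a fresh PlayerSaveGame holding the gate number, the player's capsule transform and whether the right-hand ice gauntlet is enabled, written to a single slot.
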(event OnComponentBeginOverlap(Box)
  (params (OverlappedComponent :type Primitive%20Component%20Object%20Reference) (OtherActor :type Actor%20Object%20Reference) (OtherComp :type Primitive%20Component%20Object%20Reference) (OtherBodyIndex :type Integer) (bFromSweep :type Boolean) (SweepResult :type Hit%20Result%20Structure%20%28by%20ref%29))
  ;[1 1 1] Check if we have a save game, if no, make one
  (bind _returnvalue (SaveGame|DoesSaveGameExist "PlayerSaveGame"))
  (if _returnvalue
    ;[1 1 1] Check if we're going backwards through gates, if so don't save. Also stops the same checkpoint triggering 2 saves
    (bind _returnvalue_2 (SaveGame|LoadGamefromSlot "PlayerSaveGame"))
    (bind _asplayer_save_game (Utilities|Casting|CastToPlayerSaveGame _returnvalue_2))
    (if (> (Variables|Default|GetGateNum) (Variables|/Game/Blueprints/Player/PlayerSaveGame.PlayerSaveGame_C|GetGateNum _asplayer_save_game))
      ;[1 1 1] Save
      (CallFunction|CreateSaveGameSlot))
    (else
      (CallFunction|CreateSaveGameSlot))))

(event Custom|CreateSaveGameSlot
  (bind _returnvalue (SaveGame|CreateSaveGameObject "/Game/Blueprints/Player/PlayerSaveGame.PlayerSaveGame_C"))
  ;[1 1 1] Save current gate
  (Variables|/Game/Blueprints/Player/PlayerSaveGame.PlayerSaveGame_C|SetGateNum _returnvalue (Variables|Default|GetGateNum))
  (bind _asplayer (Utilities|Casting|CastToPlayer (Game|Player|GetPlayerPawn 0)))
  ;[1 1 1] Save location & state of ice hand
  (Variables|/Game/Blueprints/Player/PlayerSaveGame.PlayerSaveGame_C|SetPlayerSaveLoc _returnvalue (Transformation|GetWorldTransform (Variables|/Script/Engine.Character|GetCapsuleComponent _asplayer)))
  (Variables|/Game/Blueprints/Player/PlayerSaveGame.PlayerSaveGame_C|SetHasIceGauntlet _returnvalue (Variables|/Script/GroupProject.HandComponent|GetbEnabled (Variables|/Script/GroupProject.PlayerBase|GetRightHand _asplayer)))
  (SaveGame|SaveGametoSlot _returnvalue "PlayerSaveGame"))

(fn ConstructionScript)
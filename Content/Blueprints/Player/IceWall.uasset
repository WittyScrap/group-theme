(event Custom|Melt
  (Components|Timeline|SetPlayRate (Variables|Default|GetMelting) (/ 1.0 (Variables|Default|GetMelt%20Time)))
  (Components|Timeline|PlayfromStart (Variables|Default|GetMelting)))

(event Custom|Create
  (bind _wall_size (Variables|Default|GetWall%20Size))
  (Components|Timeline|SetPlayRate (Variables|Default|GetCreation) (/ 1.0 (Variables|Default|GetSpawn%20Time)))
  (Transformation|SetRelativeScale3D (Variables|Default|GetWall%20Root) (Math|Vector|MakeVector (.x _wall_size) (.y _wall_size) (Variables|Default|GetWall%20Height)))
  (Components|Timeline|PlayfromStart (Variables|Default|GetCreation)))

(event EventBeginPlay
  (CallFunction|Create)
  (Utilities|FlowControl|Delay (Variables|Default|GetLifetime))
  (CallFunction|Melt))

(event Collision|EventActorBeginOverlap
  (params (OtherActor :type Actor%20Object%20Reference)))

(event EventTick
  (params (DeltaSeconds :type Float%20%28single-precision%29)))

(fn ConstructionScript)
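; TestPlayer is a test player Blueprint that creates the HUD and provides debug keys for registering deaths.
; On BeginPlay, InitiateHUD creates the BaseUI widget for player controller 0 and adds it to the viewport.
; Numpad 7, 8 and 9 cast to KillSelfGamemode and call AddDeath with long-fall, crushed and burn death names.
; The OnDied event is present but empty.
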(event EventBeginPlay
  (CallFunction|InitiateHUD "/Game/UI/BaseUI.BaseUI_C"))

(event EventOnDied
  (params (reason :type String)))

(event Input|KeyboardEvents|NumPadSeven
  (params (Key :type Key%20Structure))
  (:Pressed
    (bind _askill_self_gamemode (Utilities|Casting|CastToKillSelfGamemode (Game|GetGameMode)))
    (Default|AddDeath _askill_self_gamemode "DeathLongFall")))

(event Input|KeyboardEvents|NumPadEight
  (params (Key :type Key%20Structure))
  (:Pressed
    (bind _askill_self_gamemode (Utilities|Casting|CastToKillSelfGamemode (Game|GetGameMode)))
    (Default|AddDeath _askill_self_gamemode "DeathCrushed")))

(event Input|KeyboardEvents|NumPadNine
  (params (Key :type Key%20Structure))
  (:Pressed
    (bind _askill_self_gamemode (Utilities|Casting|CastToKillSelfGamemode (Game|GetGameMode)))
    (Default|AddDeath _askill_self_gamemode "DeathBurn")))

(fn ConstructionScript)

(fn InitiateHUD
  (params (Class :type User%20Widget%20Class%20Reference))
  (bind _returnvalue (UserInterface|CreateWidget Class (Game|GetPlayerController 0)))
  (UserInterface|Viewport|AddtoViewport _returnvalue 0))
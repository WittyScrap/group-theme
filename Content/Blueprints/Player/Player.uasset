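; Player Blueprint for a hand-based spellcaster, handling health, an unlockable second glove, ice wall placement and the game UI.
; Holding PlaceWall traces from the camera to preview a wall on upward-facing surfaces; release spawns it and animates both hands.
; Ice and fire projectile overlaps reduce health, and CheckDeath swaps in the game-over UI and notifies the controller.
; Some disconnected firing, trajectory prediction and debug code remains.
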(event OnComponentBeginOverlap(Hitbox_Projectile)
  (params (OverlappedComponent :type Primitive%20Component%20Object%20Reference) (OtherActor :type Actor%20Object%20Reference) (OtherComp :type Primitive%20Component%20Object%20Reference) (OtherBodyIndex :type Integer) (bFromSweep :type Boolean) (SweepResult :type Hit%20Result%20Structure%20%28by%20ref%29))
  ;[1 1 1] Projectile hitbox
  (Utilities|Casting|CastToProj_Ice OtherActor
    (:then
      (CallFunction|AdjPlayerHp -1e+01))
    (:CastFailed
      (Utilities|Casting|CastToProj_Fire OtherActor)
      (CallFunction|AdjPlayerHp -2e+01))))

(event Custom|FireInput
  (params (Class :type Actor%20Class%20Reference))
  ;[1 0 0] This code will never execute - it has been left here should it be needed later.
  ;;[1 0 0] Fire projectile from player-- apply cooldown
  (Utilities|FlowControl|DoOnce false :!label _label
    (:Completed
      (Utilities|FlowControl|Sequence
        (:then_0
          ;;;[1 1 1] Fire cooldown
          (Utilities|FlowControl|Delay 0.35)
          (goto _label Reset))
        (:then_1
          (Game|SpawnActorfromClass Class (Math|Transform|MakeTransform (Transformation|GetActorLocation) (Transformation|GetWorldRotation (Variables|Default|GetCamera))) "Undefined" 0 0))))))

(event Custom|Place%20Ice%20Wall
  ;[1 1 1] Spawn ice wall
  (Game|SpawnActorfromClass (Variables|Default|GetWall) (Math|Transform|MakeTransform (Variables|Default|GetWall%20Location) (Math|Rotator|MakeRotator 0.0 0.0 (.yaw (Variables|Default|GetWall%20Rotation)))) "Undefined" 0 0)
  ;[1 1 1] Play ice wall animation
  (bind _animation (Utilities|GetHandAnimation (Variables|Default|GetLeftHand)))
  (bind _animation_2 (Utilities|GetHandAnimation (Variables|Default|GetRightHand)))
  (Default|OnIceWall _animation)
  (Default|OnIceWall _animation_2))

(event EventOnPickedUp
  (params (PickedUp :type Pickup%20Object%20Reference))
  ;[1 1 1] Pickup second glove
  (Utilities|Casting|CastToSecondGlovePickup PickedUp)
  (bind _output_get (Variables|/Script/GroupProject.HandComponent|SetbEnabled (Variables|Default|GetRightHand) true))
  (Rendering|SetVisibility (Variables|Default|GetHandModelR) _output_get false))

(event EventBeginPlay
  ;[1 1 1] Add UI to screen
  (bind _returnvalue (UserInterface|CreateWidget "/Game/UI/GameUI.GameUI_C"))
  (UserInterface|Viewport|AddtoViewport _returnvalue 0)
  ;[1 1 1] Hide second hand if it is not unlocked by default
  (if (not (Variables|/Script/GroupProject.HandComponent|GetbEnabled (Variables|Default|GetRightHand)))
    (Rendering|SetVisibility (Variables|Default|GetHandModelR) false false)))

(event EventTick
  (params (DeltaSeconds :type Float%20%28single-precision%29))
  (bind _returnvalue (Transformation|GetActorForwardVector))
  (bind _cursor_marker (Variables|Default|GetCursor%20Marker))
  ;[1 1 1] Handle Ice Wall Gizmo
  (bind (_any _point _normal) (CallFunction|GetWallSpawnLocation "None" (Variables|Default|GetDisplay%20Wall%20Gizmo)))
  (Rendering|SetVisibility (Variables|Default|GetCursor%20Marker) _any false)
  (if _any
    (Transformation|SetWorldLocation _cursor_marker (CallFunction|Offset _point _normal (Variables|Default|GetCursor%20Distance)) false true)
    (Transformation|SetWorldRotation _cursor_marker (Math|Rotator|MakeRotationfromAxes (Utilities|-v _normal) (Math|Vector|CrossProduct _normal _returnvalue) _returnvalue) false false)
    (Variables|Default|SetWall%20Location _point)
    (Variables|Default|SetWall%20Rotation (Math|Rotator|MakeRotationfromAxes _returnvalue (Math|Vector|CrossProduct _normal _returnvalue) (Utilities|-v _normal)))))

(event EventOnFired
  (params (Hand :type Hand%20Component%20Object%20Reference))
  ;[1 1 1] Fire animation
  (bind _animation (Utilities|GetHandAnimation Hand))
  (Default|OnFire _animation))

(event Input|ActionEvents|InputActionPlaceWall
  (params (Key :type Key%20Structure))
  ;[1 1 1] Ice wall generation
  (:Pressed
    (if (Variables|/Script/GroupProject.HandComponent|GetbEnabled (Variables|Default|GetRightHand))
      (Variables|Default|SetDisplay%20Wall%20Gizmo true)))
  (:Released
    (if (Variables|/Script/GroupProject.HandComponent|GetbEnabled (Variables|Default|GetRightHand))
      (Variables|Default|SetDisplay%20Wall%20Gizmo false)
      (CallFunction|PlaceIceWall))))

(event Input|KeyboardEvents|NumPadZero
  (params (Key :type Key%20Structure))
  ;[1 0 0] remove me
)

(fn ConstructionScript)

(fn AdjPlayerHp
  (params (Value :type Float%20%28single-precision%29))
  ;[1 1 1] Event to adjust player points (i.e. gain or lose health)
  (if (not (Variables|Default|GetbInvincible))
    (Variables|Default|SetPlayerHealth (+ (Variables|Default|GetPlayerHealth) Value))
    (CallFunction|CheckDeath false)))

(fn CheckDeath
  (params (ForceDeath :type Boolean))
  (if (Math|Boolean|ANDBoolean (or ForceDeath (<= (Variables|Default|GetPlayerHealth) 0.0)) (not (Variables|Default|GetbInvincible)) (Variables|Default|GetbAlive))
    (Variables|Default|SetPlayerHealth 0.0)
    (Utilities|FlowControl|DoOnce false
      (:Completed
        (Utilities|FlowControl|Sequence
          (:then_0
            ;[1 1 1] Add game over UI
            (bind _returnvalue (UserInterface|CreateWidget "/Game/UI/UI_GameOver.UI_GameOver_C"))
            (UserInterface|Viewport|AddtoViewport _returnvalue 0))
          (:then_1
            ;[1 1 1] Remove base UI from view
            (bind _foundwidgets (Widget|GetAllWidgetsOfClass "/Game/UI/GameUI.GameUI_C" true))
            (for _array_element _foundwidgets
              (Widget|RemovefromParent _array_element)))
          (:then_2
            ;[1 1 1] Set player to dead on controller
            (bind _asdragon_game_player_controller (Utilities|Casting|CastToDragonGamePlayerController (Pawn|GetController)))
            (Variables|/Game/Blueprints/Global/DragonGamePlayerController.DragonGamePlayerController_C|SetPlayerAlive _asdragon_game_player_controller false)
            (Variables|Default|SetbAlive false)))))))

(fn GetWallSpawnLocation
  (params (Debug :type EDrawDebugTrace%20Enum :default "None") (Allow :type Boolean))
  (bind _camera (Variables|Default|GetCamera))
  (bind _returnvalue (Transformation|GetWorldLocation _camera))
  (if Allow
    (bind (_outhit _returnvalue_2) (Collision|LineTraceForObjects _returnvalue (+ _returnvalue (* (Math|Vector|GetForwardVector (Variables|Default|GetCamera)) 1e+06)) (LocalVariables|GetObject%20Types) false 0 Debug))
    (if _returnvalue_2
      (if (> (Math|Vector|DotProduct (.ImpactNormal (Collision|BreakHitResult _outhit)) (Math|Vector|VectorUp)) 0.5)
        (return true (+ (.ImpactPoint (Collision|BreakHitResult _outhit)) (* (.ImpactNormal (Collision|BreakHitResult _outhit)) 1.0)) (.ImpactNormal (Collision|BreakHitResult _outhit)))
        (else
          _)))
    (return false "0, 0, 0" "0, 0, 0")
    (else
      (return false "0, 0, 0" "0, 0, 0"))))

(fn Offset
  (params (X :type Vector) (Offset :type Vector) (F :type Float%20%28single-precision%29))
  (return (+ X (* Offset F))))
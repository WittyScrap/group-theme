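; Projectile actor for shots, with configurable speed, gravity, effects and sounds so different shooters such as enemies can reuse it.
; On BeginPlay it applies BaseSpeed to the projectile movement, spawns a scaled muzzle effect actor and plays the shoot sound.
; Gravity scale is applied after a short delay.
; Any hit triggers Explode, which spawns the explosion actor, plays its sound and destroys the projectile.
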(event Custom|Explode
  ;[1 1 1] Create explosion and destroy bullet
  (Game|SpawnActorfromClass (Variables|Default|GetExplosion%20Type) (Transformation|GetActorTransform) "Undefined" 0 0)
  (Audio|PlaySoundatLocation (Variables|Default|GetExplosion%20sound) (Transformation|GetActorLocation) "0, 0, 0" 1.0 1.0 0.0 0 0 0)
  (Actor|DestroyActor))

(event EventBeginPlay
  (bind _returnvalue (Transformation|GetActorTransform))
  (bind _projectilemovement (Variables|Default|GetProjectileMovement))
  (bind _basespeed (Variables|Default|GetBaseSpeed))
  ;[1 1 1] When spawned allow us to set the projectile speed for different scenarios (ie enemies using fire)
  (Variables|/Script/Engine.ProjectileMovementComponent|SetInitialSpeed _projectilemovement _basespeed)
  (Variables|/Script/Engine.ProjectileMovementComponent|SetMaxSpeed _projectilemovement _basespeed)
  ;;[1 1 1] Spawn explosion
  (Game|SpawnActorfromClass (Variables|Default|GetShooting%20Type) (Math|Transform|MakeTransform (.location _returnvalue) (.rotation _returnvalue) (* (.scale _returnvalue) (Variables|Default|GetSpawn%20Explosion%20Scale))) "Undefined" 0 0)
  (Audio|PlaySoundatLocation (Variables|Default|GetShoot%20sound) (Transformation|GetActorLocation) "0, 0, 0" 1.0 1.0 0.0 0 0 0)
  (Utilities|FlowControl|Delay 0.05)
  (Variables|/Script/Engine.ProjectileMovementComponent|SetProjectileGravityScale _projectilemovement (Variables|Default|GetGravityScale)))

(event Collision|EventHit
  (params (MyComp :type Primitive%20Component%20Object%20Reference) (Other :type Actor%20Object%20Reference) (OtherComp :type Primitive%20Component%20Object%20Reference) (bSelfMoved :type Boolean) (HitLocation :type Vector :default "0, 0, 0") (HitNormal :type Vector :default "0, 0, 0") (NormalImpulse :type Vector :default "0, 0, 0") (Hit :type Hit%20Result%20Structure%20%28by%20ref%29))
  ;[1 1 1] Consume bullet
  (CallFunction|Explode))

(fn ConstructionScript)
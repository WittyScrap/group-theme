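; Fire plant enemy that acts as a turret, continuously shooting fire projectiles toward the player.
; Every tick it rotates its VectorField component to face the first player's pawn.
; From BeginPlay an endless DelayLoop spawns Proj_Fire at a short fixed interval, positioned at FireLoc and oriented by VectorField, with no range or visibility check.
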(event EventTick
  (params (DeltaSeconds :type Float%20%28single-precision%29))
  (Transformation|SetWorldRotation (Variables|Default|GetVectorField) (Math|Rotator|FindLookatRotation (Transformation|GetWorldLocation (Variables|Default|GetVectorField)) (Transformation|GetActorLocation (Pawn|GetControlledPawn (Game|GetPlayerController 0)))) false false))

(event EventBeginPlay
  ;[1 1 1] Fire projectile
  (Utilities|DelayLoop true 0.5
    (:Loop%20Body
      (Game|SpawnActorfromClass "/Game/Blueprints/Proj_Fire.Proj_Fire_C" (Math|Transform|MakeTransform (Transformation|GetWorldLocation (Variables|Default|GetFireLoc)) (Transformation|GetWorldRotation (Variables|Default|GetVectorField))) "Undefined" 0 6e+02 0))))

(fn ConstructionScript)
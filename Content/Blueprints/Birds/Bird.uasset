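; Bird actor that flies in a straight-line heading at a set speed once SetOff is called.
; With a valid Leader it copies the leader's forward direction, otherwise it heads toward its Target location.
; Each Tick it eases rotation toward that heading with a fixed, frame-rate-dependent lerp.
; It teleports along the desired heading without sweeping, so movement ignores collision and the smoothed facing.
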(event Custom|Set%20Off
  (Variables|Default|SetStart true))

(event EventBeginPlay)

(event Collision|EventActorBeginOverlap
  (params (OtherActor :type Actor%20Object%20Reference)))

(event EventTick
  (params (DeltaSeconds :type Float%20%28single-precision%29))
  (bind _direction (CallFunction|GetFacingDirection))
  (if (Variables|Default|GetStart)
    (CallFunction|Face _direction)
    (CallFunction|Move _direction (* (Variables|Default|GetMovement%20Speed) DeltaSeconds))))

(fn ConstructionScript)

(fn GetFacingDirection
  (bind _leader (Variables|Default|GetLeader))
  (Utilities|IsValid _leader
    (:Is%20Valid
      (return (Math|Vector|Normalize (Math|Vector|GetForwardVector (Variables|Bird_C|GetDefaultSceneRoot _leader)))))
    (:Is%20Not%20Valid
      (return (Math|Vector|Normalize (- (Variables|Default|GetTarget) (Transformation|GetWorldLocation (Variables|Default|GetDefaultSceneRoot))))))))

(fn Move
  (params (Direction :type Vector) (Amount :type Float%20%28single-precision%29))
  (Transformation|SetWorldLocation (Variables|Default|GetDefaultSceneRoot) (+ (Transformation|GetWorldLocation (Variables|Default|GetDefaultSceneRoot)) (* Direction Amount)) false true))

(fn Face
  (params (Direction :type Vector))
  (Transformation|SetWorldRotation (Variables|Default|GetDefaultSceneRoot) (Math|Rotator|Lerp(Rotator) (Transformation|GetWorldRotation (Variables|Default|GetDefaultSceneRoot)) (Math|Rotator|MakeRotationfromAxes Direction (Transformation|GetActorRightVector) (Transformation|GetActorUpVector)) 0.1 true) false false))

(fn SetTarget
  (params (Target :type Vector))
  (Variables|Default|SetTarget Target))
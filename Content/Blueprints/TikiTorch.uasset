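; TikiTorch is a puzzle torch that lights with fire or ice on contact and drives element triggers.
; Overlaps on CollisionTrigger read the other component's collision object type, swap the Light material, and set the numbered trigger for Fire or unset it for Ice.
; InvertTrigger reverses that mapping.
; The State variable picks the construction-time material and, unless Unlit, applies the matching trigger on BeginPlay.
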(event OnComponentBeginOverlap(CollisionTrigger)
  (params (OverlappedComponent :type Primitive%20Component%20Object%20Reference) (OtherActor :type Actor%20Object%20Reference) (OtherComp :type Primitive%20Component%20Object%20Reference) (OtherBodyIndex :type Integer) (bFromSweep :type Boolean) (SweepResult :type Hit%20Result%20Structure%20%28by%20ref%29))
  (bind _inverttrigger (Variables|Default|GetInvertTrigger))
  (bind _elementtriggerno (Variables|Default|GetElementTriggerNo))
  (switch Utilities|FlowControl|Switch|SwitchonECollisionChannel (Collision|GetCollisionObjectType OtherComp)
    (:ECC_GameTraceChannel1
      (Rendering|Material|SetMaterial (Variables|Default|GetLight) 0 "/Game/Materials/Devtest/TestFire.TestFire")
      (if _inverttrigger
        (Class|InteractionSender|UnsetTriggers _elementtriggerno :!label _label)
        (else
          (Class|InteractionSender|SetTriggers _elementtriggerno :!label _label_2))))
    (:ECC_GameTraceChannel2
      (Rendering|Material|SetMaterial (Variables|Default|GetLight) 0 "/Game/Materials/Devtest/TestIce.TestIce")
      (if _inverttrigger
        (goto _label_2)
        (else
          (goto _label))))))

(event EventBeginPlay
  (bind _inverttrigger (Variables|Default|GetInvertTrigger))
  (bind _elementtriggerno (Variables|Default|GetElementTriggerNo))
  (switch string (Variables|Default|GetState)
    (:Fire
      (if _inverttrigger
        (Class|InteractionSender|UnsetTriggers _elementtriggerno :!label _label)
        (else
          (Class|InteractionSender|SetTriggers _elementtriggerno :!label _label_2))))
    (:Ice
      (if _inverttrigger
        (goto _label_2)
        (else
          (goto _label))))))

(fn ConstructionScript
  (bind _light (Variables|Default|GetLight))
  (switch string (Variables|Default|GetState)
    (:Unlit
      (Rendering|Material|SetMaterial _light 0 "/Game/Materials/Devtest/TestInvis.TestInvis"))
    (:Fire
      (Rendering|Material|SetMaterial _light 0 "/Game/Materials/Devtest/TestFire.TestFire"))
    (:Ice
      (Rendering|Material|SetMaterial _light 0 "/Game/Materials/Devtest/TestIce.TestIce"))))
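; Stationary plant enemy that turns toward the player and periodically fires either fire or ice projectiles while something overlaps its visibility sphere.
; While homing is on, a fast delay loop yaws the VectorField component at the player's pawn and raises its pitch with distance to compensate for range.
; A second, roughly one-second loop pulses a gate that sphere overlaps open and close, spawning projectiles at FireLoc.
; The construction script scales the sphere by VisibilityRadius.
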(event OnComponentBeginOverlap(VisSphere)
  (params (OverlappedComponent :type Primitive%20Component%20Object%20Reference) (OtherActor :type Actor%20Object%20Reference) (OtherComp :type Primitive%20Component%20Object%20Reference) (OtherBodyIndex :type Integer) (bFromSweep :type Boolean) (SweepResult :type Hit%20Result%20Structure%20%28by%20ref%29))
  (bind _projectilespd (Variables|Default|GetProjectileSpd))
  (bind _fireloc (Variables|Default|GetFireLoc))
  (bind _fireloc_2 (Variables|Default|GetFireLoc))
  (bind _returnvalue (Transformation|GetWorldLocation _fireloc))
  (bind _returnvalue_2 (Transformation|GetWorldRotation _fireloc_2))
  (bind _returnvalue_3 (Math|Transform|MakeTransform _returnvalue _returnvalue_2))
  ;[1 1 1] Visibility Radius
  ;[1 1 1] Fire projectile
  (Utilities|FlowControl|Gate true) ; enters at Open
)

(event OnComponentEndOverlap(VisSphere)
  (params (OverlappedComponent :type Primitive%20Component%20Object%20Reference) (OtherActor :type Actor%20Object%20Reference) (OtherComp :type Primitive%20Component%20Object%20Reference) (OtherBodyIndex :type Integer))
  (bind _projectilespd (Variables|Default|GetProjectileSpd))
  (bind _fireloc (Variables|Default|GetFireLoc))
  (bind _fireloc_2 (Variables|Default|GetFireLoc))
  (bind _returnvalue (Transformation|GetWorldLocation _fireloc))
  (bind _returnvalue_2 (Transformation|GetWorldRotation _fireloc_2))
  (bind _returnvalue_3 (Math|Transform|MakeTransform _returnvalue _returnvalue_2))
  ;[1 1 1] Visibility Radius
  ;[1 1 1] Fire projectile
  (Utilities|FlowControl|Gate true) ; enters at Close
)

(event Custom|Initiate_Homing
  (bind _returnvalue (Game|GetPlayerController 0))
  (bind _returnvalue_2 (Pawn|GetControlledPawn _returnvalue))
  (Utilities|DelayLoop (Variables|Default|GetHoming) 0.01
    (:Loop%20Body
      (Utilities|IsValid _returnvalue_2
        (:Is%20Valid
          (Transformation|SetWorldRotation (Variables|Default|GetVectorField) (Math|Rotator|MakeRotator 0.0 (Math|Float|Lerp 0.0 4e+01 (/ (Math|Float|Clamp(Float) (Transformation|GetDistanceTo _returnvalue_2) 0.0 6.5e+03) 6.5e+03)) (.Yaw (Math|Rotator|BreakRotator (Math|Rotator|FindLookatRotation (Transformation|GetWorldLocation (Variables|Default|GetVectorField)) (Transformation|GetActorLocation _returnvalue_2))))) false false))))))

(event EventBeginPlay
  (bind _projectilespd (Variables|Default|GetProjectileSpd))
  (bind _fireloc (Variables|Default|GetFireLoc))
  (bind _fireloc_2 (Variables|Default|GetFireLoc))
  (bind _returnvalue (Transformation|GetWorldLocation _fireloc))
  (bind _returnvalue_2 (Transformation|GetWorldRotation _fireloc_2))
  (bind _returnvalue_3 (Math|Transform|MakeTransform _returnvalue _returnvalue_2))
  (Utilities|FlowControl|Sequence
    (:then_0
      (CallFunction|InitiateHoming))
    (:then_1
      ;[1 1 1] Fire projectile
      (Utilities|DelayLoop true 0.95
        (:Loop%20Body
          (Utilities|FlowControl|Gate true
            (:Exit
              (if (Variables|Default|GetShootsFire)
                (Game|SpawnActorfromClass "/Game/Blueprints/Player/Proj_Fire.Proj_Fire_C" _returnvalue_3 "Undefined" 0 _projectilespd 0)
                (else
                  (Game|SpawnActorfromClass "/Game/Blueprints/Player/Proj_Ice.Proj_Ice_C" _returnvalue_3 "Undefined" 0 _projectilespd 0))))))))))

(fn ConstructionScript
  (bind _visibilityradius (Variables|Default|GetVisibilityRadius))
  (Transformation|SetWorldScale3D (Variables|Default|GetVisSphere) (Math|Vector|MakeVector _visibilityradius _visibilityradius _visibilityradius)))
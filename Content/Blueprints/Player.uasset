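; Player Blueprint that fires fire and ice projectiles from input.
; The ShootFire and ShootIce input actions both call a shared FireInput event with their projectile class.
; FireInput spawns that class at the actor's location facing the camera's rotation.
; A DoOnce reset after a short delay gives both projectile types one shared cooldown.
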(event Custom|FireInput
  (params (Class :type Actor%20Class%20Reference))
  ;[1 1 1] Fire projectile from player-- apply cooldown
  (Utilities|FlowControl|DoOnce false :!label _label
    (:Completed
      (Utilities|FlowControl|Sequence
        (:then_0
          ;;[1 1 1] Fire cooldown
          (Utilities|FlowControl|Delay 0.35)
          (goto _label Reset))
        (:then_1
          (Game|SpawnActorfromClass Class (Math|Transform|MakeTransform (Transformation|GetActorLocation) (Transformation|GetWorldRotation (Variables|Default|GetCamera))) "Undefined" 0 0))))))

(event Input|ActionEvents|InputActionShootFire
  (params (Key :type Key%20Structure))
  (:Pressed
    (CallFunction|FireInput "/Game/Blueprints/Proj_Fire.Proj_Fire_C")))

(event Input|ActionEvents|InputActionShootIce
  (params (Key :type Key%20Structure))
  (:Pressed
    (CallFunction|FireInput "/Game/Blueprints/Proj_Ice.Proj_Ice_C")))

(fn ConstructionScript)
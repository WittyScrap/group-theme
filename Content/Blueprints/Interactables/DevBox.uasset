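; DevBox is an interactable test box with Default, Frozen and Burned states that reacts to freeze and burn events.
; Freezing applies an ice material; burning restores a frozen box, otherwise applies fire and destroys it after a short delay.
; Original materials are cached once for resets, though every entry copies slot 0.
; The construction script applies a preset starting state, and BeginPlay reruns burning because it doesn't take effect during construction.
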(event Custom|BurnSelf
  ;[1 1 1] Events to happen on burnt
  (Rendering|Material|SetMaterial (Variables|Default|GetCube) 0 "/Game/Materials/Devtest/TestFire.TestFire")
  (Variables|Default|SetState "Burned")
  (Utilities|FlowControl|Delay 0.35)
  (Actor|DestroyActor))

(event EventBurnObject
  ;[1 1 1] Events to happen on burnt
  (if (Utilities|Enum|Equal(Enum) (Variables|Default|GetState) "Frozen")
    (CallFunction|ResetObject)
    (else
      (CallFunction|BurnSelf))))

(event EventFreezeObject
  ;[1 1 1] Events to happen on frozen
  (Rendering|Material|SetMaterial (Variables|Default|GetCube) 0 "/Game/Materials/Devtest/TestIce.TestIce")
  (Variables|Default|SetState "Frozen"))

(event EventResetObject
  ;[1 1 1] Return object to original state
  (CallFunction|ApplyDefaultMaterials)
  (Variables|Default|SetState "Default"))

(event EventBeginPlay
  (Utilities|FlowControl|Sequence
    (:then_0
      ;[1 1 1] Save our default materials
      (CallFunction|StoreDefaultMaterials))
    (:then_1
      ;[1 1 1] Burning events don't apply during construction script-- if we start burned, call burning events
      (if (Utilities|Enum|Equal(Enum) (Variables|Default|GetState) "Burned")
        (CallFunction|BurnSelf)))))

(fn ConstructionScript
  (switch string (Variables|Default|GetState)
    (:Frozen
      (CallFunction|StoreDefaultMaterials)
      (CallFunction|FreezeObject))
    (:Burned
      (CallFunction|StoreDefaultMaterials)
      (CallFunction|BurnObject))))

(fn StoreDefaultMaterials
  ;[1 1 1] Save the default materials on begin play-- we use this so we don't have to enter each material for each object
  (if (== (Utilities|Array|Length (Variables|Default|GetStoredMaterials)) 0)
    (for _index (range 0 (- (Rendering|Material|GetNumMaterials (Variables|Default|GetCube)) 1))
      (Utilities|Array|Add (Variables|Default|GetStoredMaterials) (Rendering|Material|GetMaterial (Variables|Default|GetCube) 0)))))

(fn ApplyDefaultMaterials
  ;[1 1 1] Set materials using stored reference
  (for (_array_element _array_index) (Variables|Default|GetStoredMaterials)
    (Rendering|Material|SetMaterial (Variables|Default|GetCube) _array_index _array_element)))
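; Interactable mushroom that grows when frozen and launches the player upward as a bounce pad.
; Freezing plays a Grow timeline that scales width/depth and height on separate tracks up to GrownSize, and thawing reverses it.
; BeginPlay sets the timeline's rate from GrowthTime.
; While frozen, hits from the Player with a near-vertical impact normal, checked by dot product, add a mass-independent upward impulse of Power.
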(event EventBeginPlay
  ;[1 1 1] Set animation speed
  (Components|Timeline|SetPlayRate (Variables|Default|GetGrow) (Utilities|OneOver (Variables|Default|GetGrowth%20Time))))

(event EventOnFrozen
  (params (bullet :type Actor%20Object%20Reference))
  ;[1 1 1] Growth animation
  (bind (_direction _height _width___depth) (Timeline|Grow Play)
    (:Update
      (Transformation|SetActorRelativeScale3D (Math|Vector|MakeVector (* _width___depth (Variables|Default|GetGrown%20Size)) (* _width___depth (Variables|Default|GetGrown%20Size)) (* _height (Variables|Default|GetGrown%20Size)))))))

(event EventOnThawed
  (params (bullet :type Actor%20Object%20Reference))
  ;[1 1 1] Growth animation
  (bind (_direction _height _width___depth) (Timeline|Grow Reverse)
    (:Update
      (Transformation|SetActorRelativeScale3D (Math|Vector|MakeVector (* _width___depth (Variables|Default|GetGrown%20Size)) (* _width___depth (Variables|Default|GetGrown%20Size)) (* _height (Variables|Default|GetGrown%20Size)))))))

(event Collision|EventHit
  (params (MyComp :type Primitive%20Component%20Object%20Reference) (Other :type Actor%20Object%20Reference) (OtherComp :type Primitive%20Component%20Object%20Reference) (bSelfMoved :type Boolean) (HitLocation :type Vector :default "0, 0, 0") (HitNormal :type Vector :default "0, 0, 0") (NormalImpulse :type Vector :default "0, 0, 0") (Hit :type Hit%20Result%20Structure%20%28by%20ref%29))
  ;[1 1 1] Bounce player
  (if (Utilities|Select :Index (Class|SpellActor|GetState) :TS_None false :TS_Frozen true :TS_Burned false)
    (bind _asplayer (Utilities|Casting|CastToPlayer Other))
    (if (>= (Math|Vector|DotProduct "0, 0,-1.000000" (.ImpactNormal (Collision|BreakHitResult Hit))) 0.75)
      (Physics|AddImpulse (Variables|/Script/Engine.Character|GetCharacterMovement _asplayer) (Math|Vector|MakeVector 0.0 0.0 (Variables|Default|GetPower)) true))))

(fn ConstructionScript)
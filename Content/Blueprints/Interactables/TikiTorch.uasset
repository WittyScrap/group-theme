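; A tiki torch interactable that switches between burning and iced states and drives numbered element triggers.
; Overlaps on CollisionTrigger check the other component's collision object type: Fire ignites it with looping-style randomized sound start, while Ice shows the ice and stops flame and sound.
; Each change sets or unsets ElementTriggerNo, reversed by InvertTrigger.
; BeginPlay runs the same branches from the initial State.
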(event OnComponentBeginOverlap(CollisionTrigger)
  (params (OverlappedComponent :type Primitive%20Component%20Object%20Reference) (OtherActor :type Actor%20Object%20Reference) (OtherComp :type Primitive%20Component%20Object%20Reference) (OtherBodyIndex :type Integer) (bFromSweep :type Boolean) (SweepResult :type Hit%20Result%20Structure%20%28by%20ref%29))
  (bind _inverttrigger (Variables|Default|GetInvertTrigger))
  (bind _elementtriggerno (Variables|Default|GetElementTriggerNo))
  (switch Utilities|FlowControl|Switch|SwitchonECollisionChannel (Collision|GetCollisionObjectType OtherComp)
    (:ECC_GameTraceChannel1
      (Components|Activation|SetActive (Variables|Default|GetFire) true false)
      (Rendering|SetVisibility (Variables|Default|GetIce) false false)
      (Audio|Components|Audio|Play (Variables|Default|GetFire%20Sound) (Math|Random|RandomFloatinRange 0.0 (Variables|/Script/Engine.SoundBase|GetDuration (Variables|/Script/Engine.AudioComponent|GetSound (Variables|Default|GetFire%20Sound)))))
      (if _inverttrigger
        (Class|InteractionSender|UnsetTriggers _elementtriggerno :!label _label)
        (else
          (Class|InteractionSender|SetTriggers _elementtriggerno :!label _label_2))))
    (:ECC_GameTraceChannel2
      (Components|Activation|SetActive (Variables|Default|GetFire) false false)
      (Rendering|SetVisibility (Variables|Default|GetIce) true false)
      (Audio|Components|Audio|Stop (Variables|Default|GetFire%20Sound))
      (if _inverttrigger
        (goto _label_2)
        (else
          (goto _label))))))

(event EventBeginPlay
  (bind _inverttrigger (Variables|Default|GetInvertTrigger))
  (bind _elementtriggerno (Variables|Default|GetElementTriggerNo))
  (switch string (Variables|Default|GetState)
    (:Fire
      (Components|Activation|SetActive (Variables|Default|GetFire) true false)
      (Rendering|SetVisibility (Variables|Default|GetIce) false false)
      (Audio|Components|Audio|Play (Variables|Default|GetFire%20Sound) (Math|Random|RandomFloatinRange 0.0 (Variables|/Script/Engine.SoundBase|GetDuration (Variables|/Script/Engine.AudioComponent|GetSound (Variables|Default|GetFire%20Sound)))))
      (if _inverttrigger
        (Class|InteractionSender|UnsetTriggers _elementtriggerno :!label _label)
        (else
          (Class|InteractionSender|SetTriggers _elementtriggerno :!label _label_2))))
    (:Ice
      (Components|Activation|SetActive (Variables|Default|GetFire) false false)
      (Rendering|SetVisibility (Variables|Default|GetIce) true false)
      (Audio|Components|Audio|Stop (Variables|Default|GetFire%20Sound))
      (if _inverttrigger
        (goto _label_2)
        (else
          (goto _label))))))

(fn ConstructionScript)
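; Interactable air draft plant that launches the player and puzzle elements upward when they overlap its DraftTrigger.
; A Gate opened by OnBurned and closed by OnThawed controls the draft, unless AlwaysActive bypasses it.
; Players get a vertical velocity-change impulse, while puzzle elements receive the bounce vector through an interface message.
; After a player bounce, a plant that is not AlwaysActive calls Freeze once TurnOffTime elapses.
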(event OnComponentBeginOverlap(DraftTrigger)
  (params (OverlappedComponent :type Primitive%20Component%20Object%20Reference) (OtherActor :type Actor%20Object%20Reference) (OtherComp :type Primitive%20Component%20Object%20Reference) (OtherBodyIndex :type Integer) (bFromSweep :type Boolean) (SweepResult :type Hit%20Result%20Structure%20%28by%20ref%29))
  (if (Variables|Default|GetAlwaysActive)
    _
    (else
      (Utilities|FlowControl|Gate true
        (:Exit
          _))))
  (bind _asplayer (Utilities|Casting|CastToPlayer OtherActor)
    (:then
      (Physics|AddImpulse (Variables|/Script/Engine.Character|GetCharacterMovement _asplayer) (Math|Vector|MakeVector 0.0 0.0 (Variables|Default|GetBounceForce)) true)
      (Utilities|FlowControl|Delay (Variables|Default|GetTurnOffTime))
      (if (not (Variables|Default|GetAlwaysActive))
        (Class|SpellActor|Freeze true)))
    (:CastFailed
      (if (Utilities|DoesObjectImplementInterface OtherActor "/Game/Blueprints/Lib/BPI_DragonGame_PuzzleElement.BPI_DragonGame_PuzzleElement_C")
        (Class|BPIDragonGamePuzzleElement|BounceObject(Message) OtherActor (Math|Vector|MakeVector 0.0 0.0 (Variables|Default|GetBounceForce)))))))

(event EventOnBurned
  (params (bullet :type Actor%20Object%20Reference))
  (Utilities|FlowControl|Gate true) ; enters at Open
)

(event EventOnThawed
  (params (bullet :type Actor%20Object%20Reference))
  (Utilities|FlowControl|Gate true) ; enters at Close
)

(fn ConstructionScript)
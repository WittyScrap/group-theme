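; DropBox is an interactable Blueprint whose static mesh drops to the ground below it when play begins.
; On BeginPlay it stores the mesh's location and line traces straight down for WorldStatic objects.
; On a hit, a timeline lerps the mesh from its start to the impact point, teleporting without sweep, so the fall is animated rather than physics-simulated.
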(event EventBeginPlay
  (bind _staticmesh (Variables|Default|GetStaticMesh))
  (bind _returnvalue (Transformation|GetWorldLocation _staticmesh))
  (Variables|Default|SetStartPos (Transformation|GetWorldLocation (Variables|Default|GetStaticMesh)))
  (bind (_outhit _returnvalue_2) (Collision|LineTraceForObjects _returnvalue (- _returnvalue "0, 0,5000.000000") (Utilities|Array|MakeArray "ObjectTypeQuery1") false 0 "None" true "(R=1.000000,G=0.000000,B=0.000000,A=1.000000)" "(R=0.000000,G=1.000000,B=0.000000,A=1.000000)" 0.0))
  (if _returnvalue_2
    (bind _base (Timeline|DroppingTimeline Play)
      (:Update
        (Transformation|SetWorldLocation (Variables|Default|GetStaticMesh) (Math|Vector|Lerp(Vector) (Variables|Default|GetStartPos) (.ImpactPoint (Collision|BreakHitResult _outhit)) _base) false true)))))

(fn ConstructionScript)
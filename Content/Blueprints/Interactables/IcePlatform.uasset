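; IcePlatform is a temporary platform that grows in on spawn, lasts for a timeout, then melts away.
; BeginPlay resets the countdown and plays the Spawn timeline, scaling the mesh up over SpawnTime with a Height multiplier on Z.
; Tick runs the countdown; at zero, a one-shot flag triggers the Melt timeline.
; Melt offsets the mesh along Z by MeltDistance over MeltTime, then destroys the actor.
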(event Custom|Platform%20Melted
  (Variables|Default|SetStartPosition (Transformation|GetActorLocation))
  (Components|Timeline|SetPlayRate (Variables|Default|GetMelt) (/ 1.0 (Variables|Default|GetMeltTime)))
  (bind _z_position (Timeline|Melt PlayFromStart)
    (:Update
      (Transformation|SetRelativeLocation (Variables|Debug|GetStaticMeshComponent) (Math|Vector|MakeVector (.x (Variables|Default|GetStartPosition)) (.y (Variables|Default|GetStartPosition)) (+ (* _z_position (Variables|Default|GetMeltDistance)) (.z (Variables|Default|GetStartPosition)))) false true))
    (:Finished
      (Actor|DestroyActor))))

(event EventBeginPlay
  (CallFunction|Reset)
  (Components|Timeline|SetPlayRate (Variables|Default|GetSpawn) (/ 1.0 (Variables|Default|GetSpawnTime)))
  (bind _scalevalue (Timeline|Spawn PlayFromStart)
    (:Update
      (Transformation|SetRelativeScale3D (Variables|Debug|GetStaticMeshComponent) (Math|Vector|MakeVector _scalevalue _scalevalue (* _scalevalue (Variables|Default|GetHeight)))))))

(event EventTick
  (params (DeltaSeconds :type Float%20%28single-precision%29))
  (CallFunction|TickDown DeltaSeconds))

(fn ConstructionScript)

(fn TickDown
  (params (Delta%20Time :type Float%20%28single-precision%29))
  (bind _output_get (Variables|Default|SetTimeLeft (- (Variables|Default|GetTimeLeft) Delta%20Time)))
  (if (<= _output_get 0.0)
    (Variables|Default|SetTimeLeft 0.0)
    (CallFunction|TimeoutCheck)))

(fn Reset
  (Variables|Default|SetTimeLeft (Variables|Default|GetTimeout)))

(fn TimeoutCheck
  (if (and (<= (Variables|Default|GetTimeLeft) 0.0) (not (Variables|Default|GetIsMelted)))
    (Variables|Default|SetIsMelted true)
    (CallFunction|PlatformMelted)))
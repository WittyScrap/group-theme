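; Wall tiki torch interactable that fire and ice projectiles switch between burning and frozen, driving an element trigger.
; An overlapping Projectile's collision object type selects the element, toggles the Fire effect and Ice visibility, updates the trigger, then explodes the projectile.
; Fire sets ElementTriggerNo and Ice unsets it, reversed by InvertTrigger.
; BeginPlay applies only the trigger logic for the initial State, leaving visuals untouched.
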(event OnComponentBeginOverlap(CollisionTrigger)
  (params (OverlappedComponent :type Primitive%20Component%20Object%20Reference) (OtherActor :type Actor%20Object%20Reference) (OtherComp :type Primitive%20Component%20Object%20Reference) (OtherBodyIndex :type Integer) (bFromSweep :type Boolean) (SweepResult :type Hit%20Result%20Structure%20%28by%20ref%29))
  (bind _inverttrigger (Variables|Default|GetInvertTrigger))
  (bind _elementtriggerno (Variables|Default|GetElementTriggerNo))
  (bind _asprojectile (Utilities|Casting|CastToProjectile OtherActor))
  (switch Utilities|FlowControl|Switch|SwitchonECollisionChannel (Collision|GetCollisionObjectType OtherComp)
    (:ECC_GameTraceChannel1
      (Components|Activation|SetActive (Variables|Default|GetFire) true false)
      (Rendering|SetVisibility (Variables|Default|GetIce) false false)
      (Utilities|FlowControl|Sequence
        (:then_0
          (if _inverttrigger
            (Class|InteractionSender|UnsetTriggers _elementtriggerno :!label _label)
            (else
              (Class|InteractionSender|SetTriggers _elementtriggerno :!label _label_2))))
        (:then_1
          (Default|Explode _asprojectile))))
    (:ECC_GameTraceChannel2
      (Components|Activation|SetActive (Variables|Default|GetFire) false false)
      (Rendering|SetVisibility (Variables|Default|GetIce) true false)
      (Utilities|FlowControl|Sequence
        (:then_0
          (if _inverttrigger
            (goto _label_2)
            (else
              (goto _label))))
        (:then_1
          (Default|Explode _asprojectile))))))

(event EventBeginPlay
  (bind _inverttrigger (Variables|Default|GetInvertTrigger))
  (bind _elementtriggerno (Variables|Default|GetElementTriggerNo))
  (switch string (Variables|Default|GetState)
    (:Fire
      (if _inverttrigger
        (Class|InteractionSender|UnsetTriggers _elementtriggerno :!label _label)
        (else
          (Class|InteractionSender|SetTriggers _elementtriggerno :!label _label_2))))
    (:Ice
      (if _inverttrigger
        (goto _label_2)
        (else
          (goto _label))))))

(fn ConstructionScript)
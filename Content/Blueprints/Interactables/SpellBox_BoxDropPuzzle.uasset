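; SpellBox_BoxDropPuzzle is an interactable box, named for a box drop puzzle, that leaves a scripted falling box behind when it ends play.
; On EndPlay it spawns a DropBox at the static mesh's world location, without carrying over rotation or scale.
; Its construction script sets the mesh's relative scale to the inverse of the actor's scale, so the box keeps its size when the actor is scaled.
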(event EventTick
  (params (DeltaSeconds :type Float%20%28single-precision%29))
  (|CallParentFunction DeltaSeconds) ; This node is disabled and will not be called.\nDrag off pins to build functionality.
)

(event EventEndPlay
  (params (EndPlayReason :type EEndPlayReason%20Enum :default "Destroyed"))
  ;[1 1 1] Spawn scripted falling box
  (Game|SpawnActorfromClass "/Game/Blueprints/Interactables/DropBox.DropBox_C" (Math|Conversions|ToTransform(Vector) (Transformation|GetWorldLocation (Variables|Default|GetStaticMesh))) "Undefined" 0 0))

(fn ConstructionScript
  (bind _returnvalue (Transformation|GetActorScale3D))
  (bind (_x _y _z) (Math|Vector|BreakVector _returnvalue))
  (|CallParentFunction)
  ;[1 1 1] Make sure the box doesn't scale with the object
  (Transformation|SetRelativeScale3D (Variables|Default|GetStaticMesh) (Math|Vector|MakeVector (/ 1.0 _x) (/ 1.0 _y) (/ 1.0 _z))))
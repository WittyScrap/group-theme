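; Freezable river actor that carries ice platforms downstream along a spline.
; The construction script builds overlap-only spline mesh segments, which BeginPlay registers for projectile detection.
; Created platforms are tracked until melted and moved each Tick at DriftSpeed along their sector's straight direction, without delta-time scaling.
; A backward search with dot products picks each sector as the last spline point the platform has passed.
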(event Custom|Drift
  (params (Platform :type Ice%20Platform%20Object%20Reference))
  ;[1 1 1] Drift platform
  (bind (_sector_start _sector_end) (CallFunction|GetPlatformSector Platform))
  (bind _direction (CallFunction|GetDriftDirection _sector_start _sector_end))
  (Transformation|AddActorWorldOffset Platform (* _direction (Variables|Default|GetDrift%20Speed)) false true))

(event Custom|Remove%20Platform
  (params (Platform :type Ice%20Platform%20Object%20Reference))
  ;[1 1 1] Save new platform
  ;;[1 1 1] Remove molten platforms
  (Utilities|Array|RemoveItem (Variables|Default|GetPlatforms) Platform))

(event EventBeginPlay
  ;[1 1 1] Register new components for projectile detection
  (for _array_element (Variables|Default|GetMeshData)
    (Class|FreezableLiquid|RegisterTarget _array_element)))

(event EventOnPlatformCreated
  (params (Platform :type Actor%20Object%20Reference) (location :type Vector%202D%20Structure))
  ;[1 1 1] Save new platform
  (bind _asice_platform (Utilities|Casting|CastToIcePlatform Platform))
  (Utilities|Array|Add (Variables|Default|GetPlatforms) _asice_platform)
  (EventDispatchers|BindEventtoMelted _asice_platform (delegate Custom|Remove%20Platform)))

(event EventTick
  (params (DeltaSeconds :type Float%20%28single-precision%29))
  ;[1 1 1] Apply drift function to all existing platforms
  (for _array_element (Variables|Default|GetPlatforms)
    (CallFunction|Drift _array_element)))

(fn ConstructionScript
  ;[1 1 1] Generate islands from spline
  (for _index (range 0 (- (Spline|GetNumberOfSplinePoints (Variables|Default|GetRiver%20Shape)) 2))
    (bind _returnvalue (AddComponent|AddSplineMeshComponent true))
    (Transformation|AttachComponentToComponent _returnvalue (Variables|Default|GetGeometry) "None" "KeepRelative" "KeepRelative" "KeepRelative" true)
    ;[1 1 1] Configure single islands
    (SplineMesh|SetStartandEnd _returnvalue (.Location (Spline|GetLocationandTangentatSplinePoint (Variables|Default|GetRiver%20Shape) _index "Local")) (.Tangent (Spline|GetLocationandTangentatSplinePoint (Variables|Default|GetRiver%20Shape) _index "Local")) (.Location (Spline|GetLocationandTangentatSplinePoint (Variables|Default|GetRiver%20Shape) (+ _index 1) "Local")) (.Tangent (Spline|GetLocationandTangentatSplinePoint (Variables|Default|GetRiver%20Shape) (+ _index 1) "Local")) true :!class /Script/Engine.SplineMeshComponent)
    (Collision|SetCollisionEnabled _returnvalue "QueryOnly")
    (Collision|SetCollisionResponsetoAllChannels _returnvalue "ECR_Overlap")
    (Variables|/Script/Engine.PrimitiveComponent|SetbGenerateOverlapEvents _returnvalue true)
    (Utilities|Array|Add (Variables|Default|GetMeshData) _returnvalue)))

(fn GetPlatformSector
  (params (Platform :type Ice%20Platform%20Object%20Reference))
  (bind _index (Utilities|InvertedforLoopwithBreak (- (Spline|GetNumberOfSplinePoints (Variables|Default|GetRiver%20Shape)) 2) 0 :!label _label)
    (:LoopBody
      (if (> (Math|Vector|DotProduct (.Direction (|GetReferenceFrame Platform _index)) (.Forward (|GetReferenceFrame Platform _index))) 0.0)
        (LocalVariables|SetFound%20Index _index)
        (goto _label Break)))
    (:Completed
      (return (LocalVariables|GetFound%20Index) (+ (LocalVariables|GetFound%20Index) 1)))))

(fn GetDriftDirection
  (params (Sector%20Start :type Integer) (Sector%20End :type Integer))
  (return (Math|Vector|Normalize (- (Spline|GetLocationatSplinePoint (Variables|Default|GetRiver%20Shape) Sector%20End "World") (Spline|GetLocationatSplinePoint (Variables|Default|GetRiver%20Shape) Sector%20Start "World")))))
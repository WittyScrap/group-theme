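; DevDoor is an interactable door that opens when set and closes when unset.
; OnSet and OnUnset call OpenDoor and CloseDoor, which play and reverse DoorTimeline.
; The timeline's DoorTrack lerps the relative location of the VectorField component between two Z offsets from DoorStart, sliding it vertically without sweep.
; BeginPlay teleports that component to DoorStart itself, without either offset.
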(event Custom|OpenDoor
  (bind _doorstart (Variables|Default|GetDoorStart))
  (bind _doortrack (Timeline|DoorTimeline Play)
    (:Update
      (Transformation|SetRelativeLocation (Variables|Default|GetVectorField) (Math|Vector|Lerp(Vector) (+ _doorstart "0, 0,97.199997") (+ _doorstart "0, 0,500.000000") _doortrack) false false))))

(event Custom|CloseDoor
  (bind _doorstart (Variables|Default|GetDoorStart))
  (bind _doortrack (Timeline|DoorTimeline Reverse)
    (:Update
      (Transformation|SetRelativeLocation (Variables|Default|GetVectorField) (Math|Vector|Lerp(Vector) (+ _doorstart "0, 0,97.199997") (+ _doorstart "0, 0,500.000000") _doortrack) false false))))

(event EventBeginPlay
  (Transformation|SetRelativeLocation (Variables|Default|GetVectorField) (Variables|Default|GetDoorStart) false true))

(event EventOnSet
  (CallFunction|OpenDoor))

(event EventOnUnset
  (CallFunction|CloseDoor))

(fn ConstructionScript)
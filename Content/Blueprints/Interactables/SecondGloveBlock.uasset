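; SecondGloveBlock is an interactable block that melts away when thawed.
; BeginPlay caches the Geometry component's world scale, and OnThawed plays the Melt timeline from the start.
; Melt's update logic scales Geometry's relative scale from that cached size and its finish destroys the actor, though the file marks both as never run.
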(event EventOnThawed
  (params (bullet :type Actor%20Object%20Reference))
  (Components|Timeline|PlayfromStart (Variables|Default|GetMelt)))

(event EventBeginPlay
  (Variables|Default|SetInitial%20Size (Transformation|GetWorldScale (Variables|Default|GetGeometry))))

(fn ConstructionScript)
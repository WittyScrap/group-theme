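; Test interactable physics box that can be frozen, thawed and bounced.
; Freezing stops physics simulation and gravity, zeroes velocity and applies the Ice material, while thawing re-enables physics and gravity and clears that material.
; BounceObject zeroes velocity before applying the given force as a mass-independent velocity-change impulse.
; The component hit event is empty, and a fixed upward bounce call is left unconnected.
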(event OnComponentHit(Geometry)
  (params (HitComponent :type Primitive%20Component%20Object%20Reference) (OtherActor :type Actor%20Object%20Reference) (OtherComp :type Primitive%20Component%20Object%20Reference) (NormalImpulse :type Vector :default "0, 0, 0") (Hit :type Hit%20Result%20Structure%20%28by%20ref%29)))

(event EventOnFrozen
  (params (bullet :type Actor%20Object%20Reference))
  (bind _geometry (Variables|Default|GetGeometry))
  (Physics|SetSimulatePhysics _geometry false)
  (Physics|SetEnableGravity _geometry false)
  (Rendering|Material|SetMaterial _geometry 0 "/Game/Art/Textures/Ice.Ice")
  (Physics|SetPhysicsLinearVelocity (Variables|Default|GetGeometry) "0, 0, 0" false "None"))

(event EventBounceObject
  (params (Force :type Vector :default "0, 0, 0"))
  (bind _geometry (Variables|Default|GetGeometry))
  (Physics|SetPhysicsLinearVelocity _geometry "0, 0, 0" false "None")
  (Physics|AddImpulse _geometry Force "None" true))

(event EventOnThawed
  (params (bullet :type Actor%20Object%20Reference))
  (bind _geometry (Variables|Default|GetGeometry))
  (Physics|SetSimulatePhysics _geometry true)
  (Physics|SetEnableGravity _geometry true)
  (Rendering|Material|SetMaterial _geometry 0 0))

(fn ConstructionScript)
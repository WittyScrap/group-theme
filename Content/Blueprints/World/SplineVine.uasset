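; Construction-script actor that builds a vine along an editable spline, with no runtime logic.
; For each pair of neighboring spline points it adds an X-forward spline mesh, using the end-cap mesh on the last segment and the regular vine mesh elsewhere.
; Segments take local positions and end tangents from their own points, but every start tangent is read from point 0, so joints can kink on curves.
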(event EventBeginPlay)

(event Collision|EventActorBeginOverlap
  (params (OtherActor :type Actor%20Object%20Reference)))

(event EventTick
  (params (DeltaSeconds :type Float%20%28single-precision%29)))

(fn ConstructionScript
  (bind _spline (Variables|Default|GetSpline))
  (bind _spline_2 (Variables|Default|GetSpline))
  (bind _returnvalue (Spline|GetNumberOfSplinePoints _spline))
  (for _index (range 0 (- _returnvalue 2))
    (bind _returnvalue_2 (AddComponent|AddSplineMeshComponent false (Math|Transform|MakeTransform "0,0.000000, 0")))
    (Components|StaticMesh|SetStaticMesh _returnvalue_2 (select (== _index (- _returnvalue 2)) "/Game/Blueprints/World/test-vine-end.test-vine-end" "/Game/Blueprints/World/test-vine.test-vine"))
    (SplineMesh|SetForwardAxis _returnvalue_2 "X" true)
    (SplineMesh|SetStartandEnd _returnvalue_2 (Spline|GetLocationatSplinePoint _spline_2 _index "Local") (Spline|GetTangentatSplinePoint _spline_2 0 "Local") (Spline|GetLocationatSplinePoint _spline_2 (+ _index 1) "Local") (Spline|GetTangentatSplinePoint _spline_2 (+ _index 1) "Local") true :!class /Script/Engine.SplineMeshComponent)))
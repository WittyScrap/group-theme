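; Self-moving island actor that moves its VectorField component between its start location and a relative end offset along a timeline.
; Movement can begin active on BeginPlay, while OnSet and OnUnset play or stop the timeline, with InvertTrigger swapping their roles.
; The construction script spawns a configurable child actor at a set location, passing a vertical launch strength to it if it is a BumpyMushroom.
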(event Custom|SetTimeloc
  (bind _doortrack (Timeline|DoorTimeline SetNewTime)
    (:Update
      (Transformation|SetRelativeLocation (Variables|Default|GetVectorField) (Math|Vector|Lerp(Vector) (Variables|Default|GetDoorStart) (Variables|Default|GetDoorEnd) _doortrack) true false))))

(event Custom|BeginTimeline
  (bind _doortrack (Timeline|DoorTimeline Play)
    (:Update
      (Transformation|SetRelativeLocation (Variables|Default|GetVectorField) (Math|Vector|Lerp(Vector) (Variables|Default|GetDoorStart) (Variables|Default|GetDoorEnd) _doortrack) true false))))

(event EventBeginPlay
  (Utilities|FlowControl|Sequence
    (:then_0
      (Variables|Default|SetDoorStart (Variables|/Script/Engine.SceneComponent|GetRelativeLocation (Variables|Default|GetVectorField)))
      (Variables|Default|SetDoorEnd (+ (Variables|Default|GetDoorStart) (Variables|Default|GetDoorEnd))))
    (:then_1
      (CallFunction|SetTimeloc))
    (:then_2
      (if (Variables|Default|GetStartActive)
        (CallFunction|BeginTimeline)))))

(event EventOnSet
  (if (Variables|Default|GetInvertTrigger)
    (bind _doortrack (Timeline|DoorTimeline Stop)
      (:Update
        (Transformation|SetRelativeLocation (Variables|Default|GetVectorField) (Math|Vector|Lerp(Vector) (Variables|Default|GetDoorStart) (Variables|Default|GetDoorEnd) _doortrack) true false)))
    (else
      (Timeline|DoorTimeline Play))))

(event EventOnUnset
  (if (Variables|Default|GetInvertTrigger)
    (bind _doortrack (Timeline|DoorTimeline Play)
      (:Update
        (Transformation|SetRelativeLocation (Variables|Default|GetVectorField) (Math|Vector|Lerp(Vector) (Variables|Default|GetDoorStart) (Variables|Default|GetDoorEnd) _doortrack) true false)))
    (else
      (Timeline|DoorTimeline Stop))))

(fn ConstructionScript
  (ChildActorComponent|SetChildActorClass (Variables|Default|GetChildActor) (Variables|Default|GetChild))
  (Transformation|SetRelativeLocation (Variables|Default|GetChildActor) (Variables|Default|GetChildLoc) false true)
  (if (== (Variables|/Script/Engine.ChildActorComponent|GetChildActorClass (Variables|Default|GetChildActor)) "/Game/Blueprints/Interactables/BumpyMushroom.BumpyMushroom_C")
    (bind _asbumpy_mushroom (Utilities|Casting|CastToBumpyMushroom (Variables|/Script/Engine.ChildActorComponent|GetChildActor (Variables|Default|GetChildActor))))
    (Variables|/Game/Blueprints/Interactables/BumpyMushroom.BumpyMushroom_C|SetTarget _asbumpy_mushroom (Math|Vector|MakeVector 0.0 0.0 (Variables|Default|GetBumpyMushroomStrength)))))
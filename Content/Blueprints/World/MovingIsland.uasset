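; MovingIsland is an actor that slides between its starting location and an offset end point, using logic named after a door.
; OnSet plays DoorTimeline forward through OpenDoor, and OnUnset reverses it through CloseDoor.
; BeginPlay records the start location and converts DoorEnd from a relative offset into a world position.
; The timeline track lerps between the two points, moving the whole actor by teleport without sweeping.
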(event Custom|OpenDoor
  (bind _doortrack (Timeline|DoorTimeline Play)
    (:Update
      (Transformation|SetActorLocation (Math|Vector|Lerp(Vector) (Variables|Default|GetDoorStart) (Variables|Default|GetDoorEnd) _doortrack) false true))))

(event Custom|CloseDoor
  (bind _doortrack (Timeline|DoorTimeline Reverse)
    (:Update
      (Transformation|SetActorLocation (Math|Vector|Lerp(Vector) (Variables|Default|GetDoorStart) (Variables|Default|GetDoorEnd) _doortrack) false true))))

(event EventBeginPlay
  (Variables|Default|SetDoorStart (Transformation|GetActorLocation))
  (Variables|Default|SetDoorEnd (+ (Variables|Default|GetDoorStart) (Variables|Default|GetDoorEnd))))

(event EventOnSet
  (CallFunction|OpenDoor))

(event EventOnUnset
  (CallFunction|CloseDoor))

(fn ConstructionScript)
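; Spline-driven vine Blueprint for world dressing that builds a vine with collision along an editable spline.
; The construction script calls InitVine, which divides the spline by section length and adds a spline mesh per section, fitted to local positions and tangents at its ends.
; The first section gets its own mesh, while index modulo checks swap variant meshes into later sections to break up repetition.
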(event Custom|InitVine
  (bind _spline (Variables|Default|GetSpline))
  (for _index (range 0 (Math|Float|Truncate (/ (Spline|GetSplineLength (Variables|Default|GetSpline)) (Variables|Default|GetSectionLen))))
    (Variables|Default|SetCurrentIndex _index)
    (bind _returnvalue (AddComponent|AddSplineMeshComponent false))
    (Variables|Default|SetSplineMesh _returnvalue)
    (Components|StaticMesh|SetStaticMesh (Variables|Default|GetSplineMesh) (select (== (Variables|Default|GetCurrentIndex) 0) "/Game/Art/Assets/vine1a.vine1a" (Variables|/Script/Engine.StaticMeshComponent|GetStaticMesh (Variables|Default|GetSplineMesh))))
    (if (== (Variables|Default|GetCurrentIndex) 0)
      _
      (else
        (Components|StaticMesh|SetStaticMesh (Variables|Default|GetSplineMesh) (select (== (Math|Integer|%(Integer) (Variables|Default|GetCurrentIndex) 4) 0) "/Game/Art/Assets/vine1b.vine1b" (Variables|/Script/Engine.StaticMeshComponent|GetStaticMesh (Variables|Default|GetSplineMesh))))
        (Components|StaticMesh|SetStaticMesh (Variables|Default|GetSplineMesh) (select (== (Math|Integer|%(Integer) (Variables|Default|GetCurrentIndex) 3) 0) "/Game/Art/Assets/vine1c.vine1c" (Variables|/Script/Engine.StaticMeshComponent|GetStaticMesh (Variables|Default|GetSplineMesh))))))
    (Collision|SetCollisionEnabled (Variables|Default|GetSplineMesh) "QueryAndPhysics")
    (SplineMesh|SetForwardAxis (Variables|Default|GetSplineMesh) "X" true)
    (SplineMesh|SetStartandEnd (Variables|Default|GetSplineMesh) (Spline|GetLocationatDistanceAlongSpline _spline (* (Variables|Default|GetCurrentIndex) (Variables|Default|GetSectionLen)) "Local") (Spline|GetTangentatDistanceAlongSpline _spline (* (Variables|Default|GetCurrentIndex) (Variables|Default|GetSectionLen)) "Local") (Spline|GetLocationatDistanceAlongSpline _spline (* (+ (Variables|Default|GetCurrentIndex) 1) (Variables|Default|GetSectionLen)) "Local") (Spline|GetTangentatDistanceAlongSpline _spline (* (+ (Variables|Default|GetCurrentIndex) 1) (Variables|Default|GetSectionLen)) "Local") true :!class /Script/Engine.SplineMeshComponent)))

(fn ConstructionScript
  (CallFunction|InitVine))